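; MyBasicPlayer is a player Blueprint that creates the player HUD and announces the player's current zone on screen.
; On BeginPlay it binds to a ZoneUpdated event and adds a W_Player_UI widget to the viewport.
; When the event matches its player ID, it shows a non-empty zone name as the title, then hides it after a delay.
; A flag ignores further zone updates while that title is showing.
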(event `self.ReceiveBeginPlay`
  (add `self.ZoneUpdated` (delegate `ZoneUpdated_Event`))
  ;[1 1 1] Create Player UI widget
  (bind _returnvalue (`|CreateWidget` "/Game/Blueprints/UI/W_Player_UI.W_Player_UI_C" (`GameplayStatics.GetPlayerController` 0)))
  (`UserWidget.AddToViewport` _returnvalue 0)
  (set `self.PlayerUIWidget` _returnvalue))

(event `ZoneUpdated_Event` :!signature `self.ZoneUpdated`
  (params (PlayerID :type Integer))
  (if (== PlayerID (`self.GetPlayerID`))
    ;[1 1 1] Set UI Center Title text and play animation to show/hide it
    (bind _returnvalue (`self.GetCurrentZoneName`))
    (bind _asw_player_ui (cast `/Game/Blueprints/UI/W_Player_UI` (`self.PlayerUIWidget`)))
    (bind _returnvalue_2 (`KismetTextLibrary.Conv_StringToText` _returnvalue))
    (if (`KismetTextLibrary.TextIsEmpty` _returnvalue_2)
      _
      (elif (not (`self.UICenterAnimationFlag`))
        (set `self.UICenterAnimationFlag` true)
        (`/Game/Blueprints/UI/W_Player_UI.ChangeTitleText` _asw_player_ui _returnvalue_2)
        (`/Game/Blueprints/UI/W_Player_UI.ShowTitleText` _asw_player_ui)
        (`KismetSystemLibrary.Delay` 5.0)
        (`/Game/Blueprints/UI/W_Player_UI.HideTitleText` _asw_player_ui)
        (set `self.UICenterAnimationFlag` false)))))

(event `self.ReceiveTick`
  (params (DeltaSeconds :type "Float (single-precision)")))

(fn `UserConstructionScript`)